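; Game mode that spawns and possesses the players' characters when a map begins.
; BeginPlay caches PlayerStart locations, then spawns each class in the GI_BP game instance's PlayersClasses at the same-index start, possessed by the matching player controller in game-only input.
; An empty list falls back to one Player_Strider for player 0, for debugging from the arena map.
; A separate SpawnPlayer function always spawns a given class and passes it to PossessNewCharacter.
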(event EventBeginPlay
  (bind _returnvalue (Game|GetPlayerController 0))
  (Utilities|FlowControl|Sequence
    (:then_0
      ;[0 0 0] SavePlayerSpawnsPositions
      (bind _outactors (Actor|GetAllActorsOfClass "/Script/Engine.PlayerStart"))
      (for _array_element _outactors
        (Utilities|Array|Add (Variables|Default|GetPlayerStarts) (Transformation|GetActorLocation _array_element))))
    (:then_1
      ;[0 0 0] Spawn Players and control them with the right controller
      (bind _asgi_bp (Utilities|Casting|CastToGI_BP (Game|GetGameInstance)))
      ;[1 0.8498 0] Debug from arena map
      (if (Utilities|Array|IsEmpty (Variables|/Game/GI_BP.GI_BP_C|GetPlayers_Classes _asgi_bp))
        (bind _returnvalue_2 (Game|SpawnActorfromClass "/Game/Player/Strider/Player_Strider.Player_Strider_C" (Math|Transform|MakeTransform (Utilities|Array|Get(acopy) (Variables|Default|GetPlayerStarts)) "0, 0, 0" "1.000000,1.000000,1.000000") "Undefined" 0 0))
        (Pawn|Possess _returnvalue _returnvalue_2)
        (Input|SetInputModeGameOnly _returnvalue false)
        (else
          (for (_array_element_2 _array_index) (Variables|/Game/GI_BP.GI_BP_C|GetPlayers_Classes _asgi_bp)
            (bind _returnvalue_3 (Game|SpawnActorfromClass _array_element_2 (Math|Transform|MakeTransform (Utilities|Array|Get(acopy) (Variables|Default|GetPlayerStarts) _array_index) "0, 0, 0" "1.000000,1.000000,1.000000") "Undefined" 0 0))
            (Pawn|Possess (Game|GetPlayerController _array_index) _returnvalue_3)
            (Input|SetInputModeGameOnly (Game|GetPlayerController _array_index) false)))))))

(fn ConstructionScript)

(fn SpawnPlayer
  (params (PlayerClass :type Player%20Class%20Reference))
  (bind _returnvalue (Game|SpawnActorfromClass PlayerClass (Math|Transform|MakeTransform (Variables|Default|GetStartLocations) "0, 0, 0" "1.000000,1.000000,1.000000") "AlwaysSpawn" 0 0))
  (Default|PossessNewCharacter (Variables|Default|GetPlayerController) _returnvalue))